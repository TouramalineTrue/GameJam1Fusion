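; Player character with hawk, frog and elephant fusion forms, each granting its own movement ability.
; Enhanced Input drives movement and jumping, while hard-bound keys handle dash, slam and sprite facing.
; Hawk dashes on a cooldown, frog charges jumps on Tick, and elephant slams down, polling overlaps to destroy BP_BreakableFloor.
; A/D start a looping timer that flip-flops each form's sprite materials as walk animation.
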(event `Animation`
  ; Animations
  (bind _returnvalue (`KismetSystemLibrary.K2_SetTimerDelegate` (delegate `SwapMaterial`) 0.3 true))
  (set `self.Swap timer` _returnvalue))

(event `self.ReceiveBeginPlay`
  ; get movement controller
  (bind _asplayer_controller (cast `PlayerController` (`self.GetController`)))
  (bind _returnvalue (pcsubsystem `EnhancedInputLocalPlayerSubsystem` _asplayer_controller))
  (`/Engine/EditorBlueprintResources/StandardMacros.IsValid` _returnvalue
    (:`Is Valid`
      (`EnhancedInputSubsystemInterface.AddMappingContext` _returnvalue "/Game/Player/inputs/IMC_Default.IMC_Default" 0 (struct)))))

(event `SwapMaterial`
  ; Animations
  (if (`self.HawkFusion`)
    (`/Engine/EditorBlueprintResources/StandardMacros.FlipFlop`
      (:`A`
        (`PrimitiveComponent.SetMaterial` (`self.Sprites`) 0 "/Game/Player/Sprites/Mat_Bird1.Mat_Bird1"))
      (:`B`
        (`PrimitiveComponent.SetMaterial` (`self.Sprites`) 0 "/Game/Player/Sprites/Mat_Bird2.Mat_Bird2")))
    (elif (`self.FrogFusion`)
      (`/Engine/EditorBlueprintResources/StandardMacros.FlipFlop`
        (:`A`
          (`PrimitiveComponent.SetMaterial` (`self.Sprites`) 0 "/Game/Player/Sprites/Mat_frog1.Mat_frog1"))
        (:`B`
          (`PrimitiveComponent.SetMaterial` (`self.Sprites`) 0 "/Game/Player/Sprites/Mat_frog2.Mat_frog2")))
      (elif (`self.ElephantFusion`)
        (`/Engine/EditorBlueprintResources/StandardMacros.FlipFlop`
          (:`A`
            (`PrimitiveComponent.SetMaterial` (`self.Sprites`) 0 "/Game/Player/Sprites/Mat_elephant1.Mat_elephant1"))
          (:`B`
            (`PrimitiveComponent.SetMaterial` (`self.Sprites`) 0 "/Game/Player/Sprites/Mat_Elephant2.Mat_Elephant2")))))))

(event `self.ReceiveTick`
  (params (DeltaSeconds :type "Float (single-precision)"))
  ; Jump - Charged Jump - Frog
  (if (stale `EnhancedInput|/Game/Player/inputs/IA_Jump` _output_get)
    (set `self.ChargeTime` (`KismetMathLibrary.FClamp` (+ DeltaSeconds (`self.ChargeTime`)) 0.0 (`self.MaxChargeTime`)))))

(event `EnhancedInput|/Game/Player/inputs/IA_Jump`
  (params (ActionValue :type Boolean) (ElapsedSeconds :type "Float (double-precision)") (TriggeredSeconds :type "Float (double-precision)") (InputAction :type "InputAction Object Reference" :default "/Game/Player/inputs/IA_Jump.IA_Jump"))
  ; Jump - Charged Jump - Frog
  (:`Triggered`
    (if (`self.FrogFusion`)
      (bind _output_get (set `self.IsCharging` true))
      (else
        (`self.Jump`))))
  (:`Completed`
    (`self.StopJumping`)
    (if (`self.IsCharging`)
      (`self.LaunchCharacter` (`KismetMathLibrary.MakeVector` 0.0 0.0 (/ (`KismetMathLibrary.Lerp` 500.0 1200.0 (`self.ChargeTime`)) (`self.MaxChargeTime`))))
      (`PrimitiveComponent.SetMaterial` (`self.Sprites`) 0 "/Game/Player/Sprites/Mat_Frog3.Mat_Frog3")
      (set `self.ChargeTime` 0.0)
      (set `self.IsCharging` false))))

(event `EnhancedInput|/Game/Player/inputs/IA_Move`
  (params (ActionValue :type "Vector2D Structure") (ElapsedSeconds :type "Float (double-precision)") (TriggeredSeconds :type "Float (double-precision)") (InputAction :type "InputAction Object Reference" :default "/Game/Player/inputs/IA_Move.IA_Move"))
  (bind (_returnvalue_roll _returnvalue_pitch _returnvalue_yaw) (`KismetMathLibrary.BreakRotator` (`self.GetControlRotation`)))
  (bind (_returnvalue_roll_2 _returnvalue_pitch_2 _returnvalue_yaw_2) (`KismetMathLibrary.BreakRotator` (`self.GetControlRotation`)))
  ; Moveing
  (:`Triggered`
    (`self.AddMovementInput` (`KismetMathLibrary.GetRightVector` (`KismetMathLibrary.MakeRotator` _returnvalue_roll 0.0 _returnvalue_yaw)) ActionValue_X)
    (`self.AddMovementInput` (`KismetMathLibrary.GetForwardVector` (`KismetMathLibrary.MakeRotator` 0.0 0.0 _returnvalue_yaw_2)) ActionValue_Y)))

(event `Key|D`
  (params (Key :type "Key Structure"))
  (bind _sprites (`self.Sprites`))
  (bind _sprites_2 (`self.Sprites`))
  ; Animations
  (:`Pressed`
    (`SceneComponent.K2_SetRelativeRotation` _sprites (struct :`Yaw` 90.0 :`Roll` 90.0) false false)
    (`self.Animation`))
  (:`Released`
    (if (`self.HawkFusion`)
      (`PrimitiveComponent.SetMaterial` _sprites 0 "/Game/Player/Sprites/Mat_Bird.Mat_Bird")
      (`KismetSystemLibrary.K2_ClearAndInvalidateTimerHandle` (`self.Swap timer`))
      (elif (`self.FrogFusion`)
        (`PrimitiveComponent.SetMaterial` _sprites_2 0 "/Game/Player/Sprites/Mat_frog1.Mat_frog1")
        (`KismetSystemLibrary.K2_ClearAndInvalidateTimerHandle` (`self.Swap timer`))
        (elif (`self.ElephantFusion`)
          (`PrimitiveComponent.SetMaterial` _sprites_2 0 "/Game/Player/Sprites/Mat_elephant1.Mat_elephant1")
          (`KismetSystemLibrary.K2_ClearAndInvalidateTimerHandle` (`self.Swap timer`)))))))

(event `Key|LeftShift`
  (params (Key :type "Key Structure"))
  ; Dash - Hawk Fusion
  (:`Pressed`
    (if (`self.HawkFusion`)
      (if (`self.HawkCooldown`)
        _
        (elif (`PlayerController.IsInputKeyDown` (`GameplayStatics.GetPlayerController` 0) "W")
          (`self.LaunchCharacter` (* (+ (`KismetMathLibrary.GetForwardVector` (`self.K2_GetActorRotation`)) (1.0 1.0 1.0)) (0.0 400.0 700.0)) true true)
          (set `self.HawkCooldown` true)
          (`KismetSystemLibrary.Delay` 2.0)
          (set `self.HawkCooldown` false)
          (else
            (`self.LaunchCharacter` (* (+ (`KismetMathLibrary.GetForwardVector` (`self.K2_GetActorRotation`)) (1.0 0.0 1.0)) (0.0 1500.0 200.0)) true true)
            (set `self.HawkCooldown` true)
            (`KismetSystemLibrary.Delay` 2.0)
            (set `self.HawkCooldown` false)))))))

(event `Key|A`
  (params (Key :type "Key Structure"))
  (bind _sprites (`self.Sprites`))
  ; Animations
  (:`Pressed`
    (`SceneComponent.K2_SetRelativeRotation` (`self.Sprites`) (struct :`Yaw` -90.0 :`Roll` 90.0) false false)
    (`self.Animation`))
  (:`Released`
    (if (`self.HawkFusion`)
      (`PrimitiveComponent.SetMaterial` _sprites 0 "/Game/Player/Sprites/Mat_Bird.Mat_Bird")
      (`KismetSystemLibrary.K2_ClearAndInvalidateTimerHandle` (`self.Swap timer`))
      (elif (`self.FrogFusion`)
        (`PrimitiveComponent.SetMaterial` _sprites 0 "/Game/Player/Sprites/Mat_frog1.Mat_frog1")
        (`KismetSystemLibrary.K2_ClearAndInvalidateTimerHandle` (`self.Swap timer`))
        (elif (`self.ElephantFusion`)
          (`PrimitiveComponent.SetMaterial` _sprites 0 "/Game/Player/Sprites/Mat_elephant1.Mat_elephant1")
          (`KismetSystemLibrary.K2_ClearAndInvalidateTimerHandle` (`self.Swap timer`)))))))

(event `CheckSlam`
  (bind _output (`|GetArrayItem` (`self.GetOverlappingActors` "/Game/Maps/Level_Content/BP_BreakableFloor.BP_BreakableFloor_C")))
  ; Ground Slamming - Elephant Fusion
  (`/Engine/EditorBlueprintResources/StandardMacros.IsValid` _output
    (:`Is Valid`
      (bind _asbp_breakable_floor (cast `/Game/Maps/Level_Content/BP_BreakableFloor` _output))
      (`self.K2_DestroyActor` _asbp_breakable_floor)
      (set `self.IsSlamming` false))))

(event `Key|LeftControl`
  (params (Key :type "Key Structure"))
  ; Ground Slamming - Elephant Fusion
  (:`Pressed`
    (if (`self.ElephantFusion`)
      (set `self.IsSlamming` true)
      (`self.LaunchCharacter` (0.0 0.0 -1000.0) false true)
      (`KismetSystemLibrary.K2_SetTimerDelegate` (delegate `CheckSlam`) 0.05 true))))

(fn `UserConstructionScript`)